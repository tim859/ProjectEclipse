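; BP_HealthPack is a rotating pickup that restores one health state to a survivor character.
; On overlap it casts the other actor to SurvivorChar, calls GainHealthState only if its HealthState is below the cap, then destroys itself, so a full-health survivor leaves it in place.
; Tick spins it around yaw at a frame-rate-independent YawPerSecond rate.
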(event EventBeginPlay)

(event Collision|EventActorBeginOverlap
  (params (OtherActor :type Actor%20Object%20Reference))
  (bind _assurvivor_char (Utilities|Casting|CastToSurvivorChar OtherActor))
  (if (< (Variables|/Game/BPMechanics/SurvivorChar.SurvivorChar_C|GetHealthState _assurvivor_char) 5)
    (Default|GainHealthState _assurvivor_char)
    (Actor|DestroyActor)))

(event EventTick
  (params (DeltaSeconds :type Float%20%28single-precision%29))
  (Transformation|AddActorLocalRotation (Math|Rotator|MakeRotator 0.0 0.0 (* DeltaSeconds (Variables|Default|GetYawPerSecond))) false false))

(fn ConstructionScript)