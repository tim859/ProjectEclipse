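; Fire kill chamber that torments a trapped Survivor with random gas-and-flame bursts until a timed release.
; StartFireChamber arms a Tick DoOnce that runs a smoke, random delay, fire cycle on Niagara emitters with sounds.
; ChoseFire loops it via RandomInteger(3), so the fourth emitter is never picked.
; Entering the selected emitter's box adds a hit, even before ignition; once three accumulate, the next kills, and the count never resets.
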(event OnComponentBeginOverlap(Box)
  (params (OverlappedComponent :type Primitive%20Component%20Object%20Reference) (OtherActor :type Actor%20Object%20Reference) (OtherComp :type Primitive%20Component%20Object%20Reference) (OtherBodyIndex :type Integer) (bFromSweep :type Boolean) (SweepResult :type Hit%20Result%20Structure%20%28by%20ref%29))
  ;[1 1 1] Check if player is in colider, if yes set a damage point (NOT HEALTH), Player needs 3 points of damage taken from the kill chamber to die
  (if (== (Variables|Default|GetFireToShoot) 0)
    (CallFunction|CheckPlayerFire OtherActor)))

(event OnComponentBeginOverlap(Box1)
  (params (OverlappedComponent :type Primitive%20Component%20Object%20Reference) (OtherActor :type Actor%20Object%20Reference) (OtherComp :type Primitive%20Component%20Object%20Reference) (OtherBodyIndex :type Integer) (bFromSweep :type Boolean) (SweepResult :type Hit%20Result%20Structure%20%28by%20ref%29))
  ;[1 1 1] Check if player is in colider, if yes set a damage point (NOT HEALTH), Player needs 3 points of damage taken from the kill chamber to die
  (if (== (Variables|Default|GetFireToShoot) 1)
    (CallFunction|CheckPlayerFire OtherActor)))

(event OnComponentBeginOverlap(Box2)
  (params (OverlappedComponent :type Primitive%20Component%20Object%20Reference) (OtherActor :type Actor%20Object%20Reference) (OtherComp :type Primitive%20Component%20Object%20Reference) (OtherBodyIndex :type Integer) (bFromSweep :type Boolean) (SweepResult :type Hit%20Result%20Structure%20%28by%20ref%29))
  ;[1 1 1] Check if player is in colider, if yes set a damage point (NOT HEALTH), Player needs 3 points of damage taken from the kill chamber to die
  (if (== (Variables|Default|GetFireToShoot) 2)
    (CallFunction|CheckPlayerFire OtherActor)))

(event OnComponentBeginOverlap(Box3)
  (params (OverlappedComponent :type Primitive%20Component%20Object%20Reference) (OtherActor :type Actor%20Object%20Reference) (OtherComp :type Primitive%20Component%20Object%20Reference) (OtherBodyIndex :type Integer) (bFromSweep :type Boolean) (SweepResult :type Hit%20Result%20Structure%20%28by%20ref%29))
  (if (== (Variables|Default|GetFireToShoot) 3)
    (CallFunction|CheckPlayerFire OtherActor)))

(event Custom|Again
  (bind _returnvalue (Math|Random|RandomFloatinRange 0.7 2.0))
  (bind _fire_p (Variables|Default|GetFire_P))
  (bind _fire_p1 (Variables|Default|GetFire_P1))
  (bind _fire_p2 (Variables|Default|GetFire_P2))
  (bind _fire_p3 (Variables|Default|GetFire_P3))
  (bind _returnvalue_2 (Transformation|GetWorldLocation _fire_p1))
  (bind _returnvalue_3 (Transformation|GetWorldLocation _fire_p2))
  (bind _returnvalue_4 (Transformation|GetWorldLocation _fire_p))
  (bind _returnvalue_5 (Transformation|GetWorldLocation _fire_p3))
  (if (Variables|Default|GetStartKillChamber)
    (switch int (Variables|Default|GetFireToShoot)
      (:0
        (Niagara|SetNiagaraVariable(Float) _fire_p "User.SpawnSmoke" 1.0)
        (Audio|PlaySoundatLocation "/Game/BPMechanics/KillChamberMechanic/Sounds/Electric/GasFireRelease.GasFireRelease" _returnvalue_4 "0, 0, 0" 1.0 1.0 0.0 "/Game/BPMechanics/KillChamberMechanic/Sounds/Electric/Sounds_KC.Sounds_KC" 0 0 0)
        (Utilities|FlowControl|Delay _returnvalue)
        (Niagara|SetNiagaraVariable(Float) _fire_p "User.SpawnFire" 1.0)
        (Audio|PlaySoundatLocation "/Game/BPMechanics/KillChamberMechanic/Sounds/Electric/FireBurst.FireBurst" _returnvalue_4 "0, 0, 0" 1.0 1.0 0.0 "/Game/BPMechanics/KillChamberMechanic/Sounds/Electric/Sounds_KC.Sounds_KC" 0 0 0)
        (Utilities|FlowControl|Delay 1.0)
        (CallFunction|TurnOff _fire_p)
        (CallFunction|ChoseFire))
      (:1
        (Niagara|SetNiagaraVariable(Float) _fire_p1 "User.SpawnSmoke" 1.0)
        (Audio|PlaySoundatLocation "/Game/BPMechanics/KillChamberMechanic/Sounds/Electric/GasFireRelease.GasFireRelease" _returnvalue_2 "0, 0, 0" 1.0 1.0 0.0 "/Game/BPMechanics/KillChamberMechanic/Sounds/Electric/Sounds_KC.Sounds_KC" 0 0 0)
        (Utilities|FlowControl|Delay _returnvalue)
        (Niagara|SetNiagaraVariable(Float) _fire_p1 "User.SpawnFire" 1.0)
        (Audio|PlaySoundatLocation "/Game/BPMechanics/KillChamberMechanic/Sounds/Electric/FireBurst.FireBurst" _returnvalue_2 "0, 0, 0" 1.0 1.0 0.0 "/Game/BPMechanics/KillChamberMechanic/Sounds/Electric/Sounds_KC.Sounds_KC" 0 0 0)
        (Utilities|FlowControl|Delay 1.0)
        (CallFunction|TurnOff _fire_p1)
        (CallFunction|ChoseFire))
      (:2
        (Niagara|SetNiagaraVariable(Float) _fire_p2 "User.SpawnSmoke" 1.0)
        (Audio|PlaySoundatLocation "/Game/BPMechanics/KillChamberMechanic/Sounds/Electric/GasFireRelease.GasFireRelease" _returnvalue_3 "0, 0, 0" 1.0 1.0 0.0 "/Game/BPMechanics/KillChamberMechanic/Sounds/Electric/Sounds_KC.Sounds_KC" 0 0 0)
        (Utilities|FlowControl|Delay _returnvalue)
        (Niagara|SetNiagaraVariable(Float) _fire_p2 "User.SpawnFire" 1.0)
        (Audio|PlaySoundatLocation "/Game/BPMechanics/KillChamberMechanic/Sounds/Electric/FireBurst.FireBurst" _returnvalue_3 "0, 0, 0" 1.0 1.0 0.0 "/Game/BPMechanics/KillChamberMechanic/Sounds/Electric/Sounds_KC.Sounds_KC" 0 0 0)
        (Utilities|FlowControl|Delay 1.0)
        (CallFunction|TurnOff _fire_p2)
        (CallFunction|ChoseFire))
      (:3
        (Niagara|SetNiagaraVariable(Float) _fire_p3 "User.SpawnSmoke" 1.0)
        (Audio|PlaySoundatLocation "/Game/BPMechanics/KillChamberMechanic/Sounds/Electric/GasFireRelease.GasFireRelease" _returnvalue_5 "0, 0, 0" 1.0 1.0 0.0 "/Game/BPMechanics/KillChamberMechanic/Sounds/Electric/Sounds_KC.Sounds_KC" 0 0 0)
        (Utilities|FlowControl|Delay _returnvalue)
        (Niagara|SetNiagaraVariable(Float) _fire_p3 "User.SpawnFire" 1.0)
        (Audio|PlaySoundatLocation "/Game/BPMechanics/KillChamberMechanic/Sounds/Electric/FireBurst.FireBurst" _returnvalue_5 "0, 0, 0" 1.0 1.0 0.0 "/Game/BPMechanics/KillChamberMechanic/Sounds/Electric/Sounds_KC.Sounds_KC" 0 0 0)
        (Utilities|FlowControl|Delay 1.0)
        (CallFunction|TurnOff _fire_p3)
        (CallFunction|ChoseFire)))))

(event Custom|RestartChamber
  (bind _returnvalue (Math|Random|RandomFloatinRange 0.7 2.0))
  (bind _fire_p (Variables|Default|GetFire_P))
  (bind _fire_p1 (Variables|Default|GetFire_P1))
  (bind _fire_p2 (Variables|Default|GetFire_P2))
  (bind _fire_p3 (Variables|Default|GetFire_P3))
  (bind _returnvalue_2 (Transformation|GetWorldLocation _fire_p1))
  (bind _returnvalue_3 (Transformation|GetWorldLocation _fire_p2))
  (bind _returnvalue_4 (Transformation|GetWorldLocation _fire_p))
  (bind _returnvalue_5 (Transformation|GetWorldLocation _fire_p3))
  ;[1 1 1] set to trueand call restartchamber once,  to start kill chamber everytime
  (Utilities|FlowControl|Sequence
    (:then_0
      (Utilities|FlowControl|DoOnce false :!label _label
        (:Completed
          (Utilities|FlowControl|Delay 3e+01)
          (CallFunction|ReleaseSurvivor (Variables|Default|GetSurvivor))
          (goto _label Reset))))
    (:then_1
      (Utilities|FlowControl|DoOnce false) ; enters at Reset
    )))

(event EventBeginPlay
  (Variables|Default|SetFire_Particles (Utilities|Array|MakeArray (Variables|Default|GetFire_P) (Variables|Default|GetFire_P1) (Variables|Default|GetFire_P2) (Variables|Default|GetFire_P3)))
  (for _array_element (Variables|Default|GetFire_Particles)
    (CallFunction|TurnOff _array_element)))

(event EventTick
  (params (DeltaSeconds :type Float%20%28single-precision%29))
  (bind _returnvalue (Math|Random|RandomFloatinRange 0.7 2.0))
  (bind _fire_p (Variables|Default|GetFire_P))
  (bind _fire_p1 (Variables|Default|GetFire_P1))
  (bind _fire_p2 (Variables|Default|GetFire_P2))
  (bind _fire_p3 (Variables|Default|GetFire_P3))
  (bind _returnvalue_2 (Transformation|GetWorldLocation _fire_p1))
  (bind _returnvalue_3 (Transformation|GetWorldLocation _fire_p2))
  (bind _returnvalue_4 (Transformation|GetWorldLocation _fire_p))
  (bind _returnvalue_5 (Transformation|GetWorldLocation _fire_p3))
  (if (Variables|Default|GetStartKillChamber)
    (Utilities|FlowControl|DoOnce false
      (:Completed
        (switch int (Variables|Default|GetFireToShoot)
          (:0
            (Niagara|SetNiagaraVariable(Float) _fire_p "User.SpawnSmoke" 1.0)
            (Audio|PlaySoundatLocation "/Game/BPMechanics/KillChamberMechanic/Sounds/Electric/GasFireRelease.GasFireRelease" _returnvalue_4 "0, 0, 0" 1.0 1.0 0.0 "/Game/BPMechanics/KillChamberMechanic/Sounds/Electric/Sounds_KC.Sounds_KC" 0 0 0)
            (Utilities|FlowControl|Delay _returnvalue)
            (Niagara|SetNiagaraVariable(Float) _fire_p "User.SpawnFire" 1.0)
            (Audio|PlaySoundatLocation "/Game/BPMechanics/KillChamberMechanic/Sounds/Electric/FireBurst.FireBurst" _returnvalue_4 "0, 0, 0" 1.0 1.0 0.0 "/Game/BPMechanics/KillChamberMechanic/Sounds/Electric/Sounds_KC.Sounds_KC" 0 0 0)
            (Utilities|FlowControl|Delay 1.0)
            (CallFunction|TurnOff _fire_p)
            (CallFunction|ChoseFire))
          (:1
            (Niagara|SetNiagaraVariable(Float) _fire_p1 "User.SpawnSmoke" 1.0)
            (Audio|PlaySoundatLocation "/Game/BPMechanics/KillChamberMechanic/Sounds/Electric/GasFireRelease.GasFireRelease" _returnvalue_2 "0, 0, 0" 1.0 1.0 0.0 "/Game/BPMechanics/KillChamberMechanic/Sounds/Electric/Sounds_KC.Sounds_KC" 0 0 0)
            (Utilities|FlowControl|Delay _returnvalue)
            (Niagara|SetNiagaraVariable(Float) _fire_p1 "User.SpawnFire" 1.0)
            (Audio|PlaySoundatLocation "/Game/BPMechanics/KillChamberMechanic/Sounds/Electric/FireBurst.FireBurst" _returnvalue_2 "0, 0, 0" 1.0 1.0 0.0 "/Game/BPMechanics/KillChamberMechanic/Sounds/Electric/Sounds_KC.Sounds_KC" 0 0 0)
            (Utilities|FlowControl|Delay 1.0)
            (CallFunction|TurnOff _fire_p1)
            (CallFunction|ChoseFire))
          (:2
            (Niagara|SetNiagaraVariable(Float) _fire_p2 "User.SpawnSmoke" 1.0)
            (Audio|PlaySoundatLocation "/Game/BPMechanics/KillChamberMechanic/Sounds/Electric/GasFireRelease.GasFireRelease" _returnvalue_3 "0, 0, 0" 1.0 1.0 0.0 "/Game/BPMechanics/KillChamberMechanic/Sounds/Electric/Sounds_KC.Sounds_KC" 0 0 0)
            (Utilities|FlowControl|Delay _returnvalue)
            (Niagara|SetNiagaraVariable(Float) _fire_p2 "User.SpawnFire" 1.0)
            (Audio|PlaySoundatLocation "/Game/BPMechanics/KillChamberMechanic/Sounds/Electric/FireBurst.FireBurst" _returnvalue_3 "0, 0, 0" 1.0 1.0 0.0 "/Game/BPMechanics/KillChamberMechanic/Sounds/Electric/Sounds_KC.Sounds_KC" 0 0 0)
            (Utilities|FlowControl|Delay 1.0)
            (CallFunction|TurnOff _fire_p2)
            (CallFunction|ChoseFire))
          (:3
            (Niagara|SetNiagaraVariable(Float) _fire_p3 "User.SpawnSmoke" 1.0)
            (Audio|PlaySoundatLocation "/Game/BPMechanics/KillChamberMechanic/Sounds/Electric/GasFireRelease.GasFireRelease" _returnvalue_5 "0, 0, 0" 1.0 1.0 0.0 "/Game/BPMechanics/KillChamberMechanic/Sounds/Electric/Sounds_KC.Sounds_KC" 0 0 0)
            (Utilities|FlowControl|Delay _returnvalue)
            (Niagara|SetNiagaraVariable(Float) _fire_p3 "User.SpawnFire" 1.0)
            (Audio|PlaySoundatLocation "/Game/BPMechanics/KillChamberMechanic/Sounds/Electric/FireBurst.FireBurst" _returnvalue_5 "0, 0, 0" 1.0 1.0 0.0 "/Game/BPMechanics/KillChamberMechanic/Sounds/Electric/Sounds_KC.Sounds_KC" 0 0 0)
            (Utilities|FlowControl|Delay 1.0)
            (CallFunction|TurnOff _fire_p3)
            (CallFunction|ChoseFire)))))
    (else
      (Variables|Default|SetTime 0.0))))

(fn ConstructionScript)

(fn TurnOff
  (params (TargetVFX :type Niagara%20Component%20Object%20Reference))
  (Niagara|SetNiagaraVariable(Float) TargetVFX "User.SpawnSmoke" 0.0)
  (Niagara|SetNiagaraVariable(Float) TargetVFX "User.SpawnFire" 0.0))

(fn ChoseFire
  (Variables|Default|SetFireToShoot (Math|Random|RandomInteger 3))
  (CallFunction|Again))

(fn CheckPlayerFire
  (params (Object :type Object%20Object%20Reference))
  (bind _firehealth (Variables|Default|GetFireHealth))
  (bind _assurvivor_char (Utilities|Casting|CastToSurvivorChar Object))
  (if (>= _firehealth 3)
    (Default|KillSurvivor _assurvivor_char)
    (else
      (Math|Integer|IncrementInt _firehealth
        (:%20%20
          (Development|PrintString "hit"))))))

(fn StartFireChamber
  (params (Survivor :type Survivor%20Char%20Object%20Reference))
  (Variables|Default|SetSurvivor Survivor)
  (Variables|Default|SetStartKillChamber true)
  (CallFunction|RestartChamber))

(fn ReleaseSurvivor
  (params (Survivor :type Survivor%20Char%20Object%20Reference))
  (Variables|Default|SetStartKillChamber false)
  (Default|ResetSurvivor Survivor))