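; Electricity kill chamber that traps a survivor with randomly firing arcs, then resets and releases them after 30 seconds.
; Once started, it loops: charge sounds at one of three point pairs, a random delay, a brief Niagara arc driven by user parameters, then a random next pair.
; Overlapping the box matching the selected pair adds a hit, or kills the survivor once three hits have accumulated.
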(event OnComponentBeginOverlap(Box)
  (params (OverlappedComponent :type Primitive%20Component%20Object%20Reference) (OtherActor :type Actor%20Object%20Reference) (OtherComp :type Primitive%20Component%20Object%20Reference) (OtherBodyIndex :type Integer) (bFromSweep :type Boolean) (SweepResult :type Hit%20Result%20Structure%20%28by%20ref%29))
  ;[1 1 1] Check colision
  (if (== (Variables|Default|GetElectricityToShoot) 0)
    (CallFunction|CheckPlayerElectricity OtherActor)))

(event OnComponentBeginOverlap(Box1)
  (params (OverlappedComponent :type Primitive%20Component%20Object%20Reference) (OtherActor :type Actor%20Object%20Reference) (OtherComp :type Primitive%20Component%20Object%20Reference) (OtherBodyIndex :type Integer) (bFromSweep :type Boolean) (SweepResult :type Hit%20Result%20Structure%20%28by%20ref%29))
  ;[1 1 1] Check colision
  (if (== (Variables|Default|GetElectricityToShoot) 1)
    (CallFunction|CheckPlayerElectricity OtherActor)))

(event OnComponentBeginOverlap(Box2)
  (params (OverlappedComponent :type Primitive%20Component%20Object%20Reference) (OtherActor :type Actor%20Object%20Reference) (OtherComp :type Primitive%20Component%20Object%20Reference) (OtherBodyIndex :type Integer) (bFromSweep :type Boolean) (SweepResult :type Hit%20Result%20Structure%20%28by%20ref%29))
  ;[1 1 1] Check colision
  (if (== (Variables|Default|GetElectricityToShoot) 2)
    (CallFunction|CheckPlayerElectricity OtherActor)))

(event Custom|Again
  (bind _returnvalue (Math|Random|RandomFloatinRange 0.7 1.5))
  (bind _electricity (Variables|Default|GetElectricity))
  (bind _electricity_2 (Variables|Default|GetElectricity))
  (bind _point2_start (Variables|Default|GetPoint2_Start))
  (bind _point2_end (Variables|Default|GetPoint2_End))
  (bind _point3_start (Variables|Default|GetPoint3_Start))
  (bind _point3_end (Variables|Default|GetPoint3_End))
  (bind _electricity_3 (Variables|Default|GetElectricity))
  (bind _point1_start (Variables|Default|GetPoint1_Start))
  (bind _point1_end (Variables|Default|GetPoint1_End))
  (if (Variables|Default|GetStart%20Kill%20Chamber)
    (switch int (Variables|Default|GetElectricityToShoot)
      (:0
        (CallFunction|PlayChargeSounds _point1_start _point1_end)
        (Utilities|FlowControl|Delay _returnvalue)
        (Transformation|SetWorldLocation _electricity_3 (Transformation|GetWorldLocation _point1_start) false true)
        (Niagara|SetNiagaraVariable(Vector3) _electricity_3 "User.EndPoint" (Transformation|GetWorldLocation _point1_end))
        (CallFunction|SpawnElect)
        ;[1 1 1] StopChargeShader
        (Utilities|FlowControl|Delay 0.5)
        (CallFunction|StopElectricity)
        (CallFunction|ChoseElectricity))
      (:1
        (CallFunction|PlayChargeSounds _point2_start _point2_end)
        (Utilities|FlowControl|Delay _returnvalue)
        (Transformation|SetWorldLocation _electricity_2 (Transformation|GetWorldLocation _point2_start) false true)
        (Niagara|SetNiagaraVariable(Vector3) _electricity_2 "User.EndPoint" (Transformation|GetWorldLocation _point2_end))
        (CallFunction|SpawnElect)
        (Utilities|FlowControl|Delay 0.5)
        (CallFunction|StopElectricity)
        (CallFunction|ChoseElectricity))
      (:2
        (CallFunction|PlayChargeSounds _point3_start _point3_end)
        (Utilities|FlowControl|Delay _returnvalue)
        (Transformation|SetWorldLocation _electricity (Transformation|GetWorldLocation _point3_start) false true)
        (Niagara|SetNiagaraVariable(Vector3) _electricity "User.EndPoint" (Transformation|GetWorldLocation _point3_end))
        (CallFunction|SpawnElect)
        (Utilities|FlowControl|Delay 0.5)
        (CallFunction|StopElectricity)
        (CallFunction|ChoseElectricity)))))

(event Custom|RestartChamber
  (bind _returnvalue (Math|Random|RandomFloatinRange 0.7 1.5))
  (bind _electricity (Variables|Default|GetElectricity))
  (bind _electricity_2 (Variables|Default|GetElectricity))
  (bind _point2_start (Variables|Default|GetPoint2_Start))
  (bind _point2_end (Variables|Default|GetPoint2_End))
  (bind _point3_start (Variables|Default|GetPoint3_Start))
  (bind _point3_end (Variables|Default|GetPoint3_End))
  (bind _electricity_3 (Variables|Default|GetElectricity))
  (bind _point1_start (Variables|Default|GetPoint1_Start))
  (bind _point1_end (Variables|Default|GetPoint1_End))
  ;[1 1 1] set to trueand call restartchamber once,  to start kill chamber everytime
  (Utilities|FlowControl|Sequence
    (:then_0
      (Utilities|FlowControl|DoOnce false :!label _label
        (:Completed
          (Utilities|FlowControl|Delay 3e+01)
          (CallFunction|ReleaseSurvivor (Variables|Default|GetSurvivor))
          (goto _label Reset))))
    (:then_1
      (Utilities|FlowControl|DoOnce false) ; enters at Reset
    )))

(event EventTick
  (params (DeltaSeconds :type Float%20%28single-precision%29))
  (bind _returnvalue (Math|Random|RandomFloatinRange 0.7 1.5))
  (bind _electricity (Variables|Default|GetElectricity))
  (bind _electricity_2 (Variables|Default|GetElectricity))
  (bind _point2_start (Variables|Default|GetPoint2_Start))
  (bind _point2_end (Variables|Default|GetPoint2_End))
  (bind _point3_start (Variables|Default|GetPoint3_Start))
  (bind _point3_end (Variables|Default|GetPoint3_End))
  (bind _electricity_3 (Variables|Default|GetElectricity))
  (bind _point1_start (Variables|Default|GetPoint1_Start))
  (bind _point1_end (Variables|Default|GetPoint1_End))
  (if (Variables|Default|GetStart%20Kill%20Chamber)
    (Utilities|FlowControl|DoOnce false
      (:Completed
        (switch int (Variables|Default|GetElectricityToShoot)
          (:0
            (CallFunction|PlayChargeSounds _point1_start _point1_end)
            (Utilities|FlowControl|Delay _returnvalue)
            (Transformation|SetWorldLocation _electricity_3 (Transformation|GetWorldLocation _point1_start) false true)
            (Niagara|SetNiagaraVariable(Vector3) _electricity_3 "User.EndPoint" (Transformation|GetWorldLocation _point1_end))
            (CallFunction|SpawnElect)
            ;[1 1 1] StopChargeShader
            (Utilities|FlowControl|Delay 0.5)
            (CallFunction|StopElectricity)
            (CallFunction|ChoseElectricity))
          (:1
            (CallFunction|PlayChargeSounds _point2_start _point2_end)
            (Utilities|FlowControl|Delay _returnvalue)
            (Transformation|SetWorldLocation _electricity_2 (Transformation|GetWorldLocation _point2_start) false true)
            (Niagara|SetNiagaraVariable(Vector3) _electricity_2 "User.EndPoint" (Transformation|GetWorldLocation _point2_end))
            (CallFunction|SpawnElect)
            (Utilities|FlowControl|Delay 0.5)
            (CallFunction|StopElectricity)
            (CallFunction|ChoseElectricity))
          (:2
            (CallFunction|PlayChargeSounds _point3_start _point3_end)
            (Utilities|FlowControl|Delay _returnvalue)
            (Transformation|SetWorldLocation _electricity (Transformation|GetWorldLocation _point3_start) false true)
            (Niagara|SetNiagaraVariable(Vector3) _electricity "User.EndPoint" (Transformation|GetWorldLocation _point3_end))
            (CallFunction|SpawnElect)
            (Utilities|FlowControl|Delay 0.5)
            (CallFunction|StopElectricity)
            (CallFunction|ChoseElectricity)))))
    (else
      (Variables|Default|SetTime 0.0))))

(event EventBeginPlay
  (CallFunction|StopElectricity))

(fn ConstructionScript)

(fn SpawnElect
  (Niagara|SetNiagaraVariable(Float) (Variables|Default|GetElectricity) "User.SpawnElectricity" 1.0)
  (Audio|Components|Audio|Play (Variables|Default|GetAudio) 0.0))

(fn ChoseElectricity
  (Variables|Default|SetElectricityToShoot (Math|Random|RandomInteger 3))
  (CallFunction|Again))

(fn StopElectricity
  (Niagara|SetNiagaraVariable(Float) (Variables|Default|GetElectricity) "User.SpawnElectricity" 0.0))

(fn PlayChargeSounds
  (params (Local1 :type Static%20Mesh%20Component%20Object%20Reference) (Local2 :type Static%20Mesh%20Component%20Object%20Reference))
  (bind _returnvalue (Math|Random|RandomFloatinRange 0.9 1.0))
  (Audio|PlaySoundatLocation "/Game/BPMechanics/KillChamberMechanic/Sounds/Electric/ElectricityCharge.ElectricityCharge" (Transformation|GetWorldLocation Local1) "0, 0, 0" _returnvalue _returnvalue 0.0 "/Game/BPMechanics/KillChamberMechanic/Sounds/Electric/Sounds_KC.Sounds_KC" 0 0 0)
  (Audio|PlaySoundatLocation "/Game/BPMechanics/KillChamberMechanic/Sounds/Electric/ElectricityCharge.ElectricityCharge" (Transformation|GetWorldLocation Local2) "0, 0, 0" _returnvalue _returnvalue 0.0 "/Game/BPMechanics/KillChamberMechanic/Sounds/Electric/Sounds_KC.Sounds_KC" 0 0 0))

(fn CheckPlayerElectricity
  (params (Object :type Object%20Object%20Reference))
  (bind _electricityhealth (Variables|Default|GetElectricityHealth))
  (bind _assurvivor_char (Utilities|Casting|CastToSurvivorChar Object))
  (if (>= _electricityhealth 3)
    (Default|KillSurvivor _assurvivor_char)
    (else
      (Math|Integer|IncrementInt _electricityhealth
        (:%20%20
          (Development|PrintString "hit"))))))

(fn StartElectricityChamber
  (params (Survivor :type Survivor%20Char%20Object%20Reference))
  (Variables|Default|SetSurvivor Survivor)
  (Variables|Default|SetStart%20Kill%20Chamber true)
  (CallFunction|RestartChamber))

(fn ReleaseSurvivor
  (params (Survivor :type Survivor%20Char%20Object%20Reference))
  (Variables|Default|SetStart%20Kill%20Chamber false)
  (Default|ResetSurvivor Survivor))