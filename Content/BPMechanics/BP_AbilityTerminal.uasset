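; Hackable terminal actor where the player holds the use key inside its overlap to start a timing minigame that unlocks BP_MainLabDoor.
; Each round rotates a target to a random angle, then sweeps a pointer in alternating directions until a key press or timeout triggers a tolerance check.
; Three wins unlock the door and two losses reset the terminal.
; Tick drives the game, timelines animate meshes, and the ServerSide event is empty.
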(event Custom|Minigame
  (params (Server%20side%20minigame :type Boolean))
  (bind _scalearrayobjtimeline (Variables|Default|GetScaleArrayObjTimeLine))
  ;[1 1 1] MiniGame
  (if (and Server%20side%20minigame (Variables|Default|GetArrayScaleDone))
    (if (not (Class|KismetMathLibrary|XORBoolean (< (Variables|Default|GetWins) 3) (< (Variables|Default|GetLoss) 2)))
      ;;[1 1 1] 4 rounds or mini game as player needs 3 win with a limit of 2 loses
      (switch int (+ (Variables|Default|GetWins) (Variables|Default|GetLoss))
        (:0
          (Utilities|FlowControl|Sequence
            (:then_0
              (Utilities|FlowControl|DoOnce false
                (:Completed
                  (Variables|Default|Settarget%20Set false)
                  (Variables|Default|SetPressed false)
                  (Variables|Default|SettargetRotPos (Math|Random|RandomFloatinRange 5e+01 3.2e+02))
                  (Variables|Default|SetObjScaleDone false))))
            (:then_1
              (CallFunction|1RoundMiniGameClockWise))))
        (:1
          (Utilities|FlowControl|Sequence
            (:then_0
              (Utilities|FlowControl|DoOnce false
                (:Completed
                  (Variables|Default|Settarget%20Set false)
                  (Variables|Default|SetPressed false)
                  (Variables|Default|SettargetRotPos (Math|Random|RandomFloatinRange -5e+01 -3.2e+02))
                  (Variables|Default|SetObjScaleDone false))))
            (:then_1
              (CallFunction|1RoundMiniGameAntiClockWise))))
        (:2
          (Utilities|FlowControl|Sequence
            (:then_0
              (Utilities|FlowControl|DoOnce false
                (:Completed
                  (Variables|Default|Settarget%20Set false)
                  (Variables|Default|SetPressed false)
                  (Variables|Default|SettargetRotPos (Math|Random|RandomFloatinRange 5e+01 3.2e+02))
                  (Variables|Default|SetObjScaleDone false))))
            (:then_1
              (CallFunction|1RoundMiniGameClockWise))))
        (:3
          (Utilities|FlowControl|Sequence
            (:then_0
              (Utilities|FlowControl|DoOnce false
                (:Completed
                  (Variables|Default|Settarget%20Set false)
                  (Variables|Default|SetPressed false)
                  (Variables|Default|SettargetRotPos (Math|Random|RandomFloatinRange -5e+01 -3.2e+02))
                  (Variables|Default|SetObjScaleDone false))))
            (:then_1
              (CallFunction|1RoundMiniGameAntiClockWise)))))
      (elif (== (Variables|Default|GetWins) 3)
        (Development|PrintString "YOU WIN!!!")
        ;;[1 1 1] Telling Main door, terminal is unlocked
        (bind _returnvalue (Actor|GetActorOfClass "/Game/BPMechanics/BP_MainLabDoor.BP_MainLabDoor_C"))
        (bind _asbp_main_lab_door (Utilities|Casting|CastToBP_MainLabDoor _returnvalue))
        (Default|TellTerminalIsUnlocked _asbp_main_lab_door)
        (Variables|Default|SetSTOP true)
        (else
          (Development|PrintString "you lose")
          (Components|Timeline|PlayfromStart (Variables|Default|GetResetTerminalTimeLine))
          (Variables|Default|SetSTOP true))))
    (elif (not (Audio|Components|Audio|IsPlaying _scalearrayobjtimeline))
      (Components|Timeline|PlayfromStart _scalearrayobjtimeline))))

(event Custom|ServerSide
  (params (Input :type Boolean) (Minigame :type Boolean)))

(event Custom|InputDelay
  (params (ButtonPressed :type Boolean))
  (bind _playercontrollerreference (Variables|Default|GetplayerControllerReference))
  ;[1 1 1] Playing MiniGame after using for X duration
  (if ButtonPressed
    (Utilities|IsValid _playercontrollerreference
      (:Is%20Valid
        (Variables|Default|SetcurrentCompletion (Class|PlayerController|GetInputKeyTimeDown _playercontrollerreference (Variables|Default|GetuseKey)))
        (if (>= (Variables|Default|GetcurrentCompletion) (Variables|Default|GetmaxCompletion))
          (bind _output_get (Variables|Default|SetMiniGamePlay true))
          (Development|PrintString (Utilities|String|ToString(Boolean) _output_get)))))))

(event EventBeginPlay
  ;[1 1 1] Make Array for mesh of terminal components
  (bind _output_get (Variables|Default|SetTerminalComponent (Utilities|Array|MakeArray (Variables|Default|GetTerminal_Unreal_With_MiniGame_Lose_Circle_1) (Variables|Default|GetTerminal_Unreal_With_MiniGame_Lose_Circle_2) (Variables|Default|GetTerminal_Unreal_With_MiniGame_Win_Circle_1) (Variables|Default|GetTerminal_Unreal_With_MiniGame_Win_Circle_2) (Variables|Default|GetTerminal_Unreal_With_MiniGame_Win_Circle_3) (Variables|Default|GetTerminal_Unreal_With_MiniGame_Target) (Variables|Default|GetTerminal_Unreal_With_MiniGame_Pointer))))
  ;[1 1 1] Make Array for mesh of points won
  (bind _output_get_2 (Variables|Default|SetAttemptsWinPoint (Utilities|Array|MakeArray (Variables|Default|GetTerminal_Unreal_With_MiniGame_Win_Point_1) (Variables|Default|GetTerminal_Unreal_With_MiniGame_Win_Point_2) (Variables|Default|GetTerminal_Unreal_With_MiniGame_Win_Point_3))))
  ;[1 1 1] Make Array for mesh of points lost
  (bind _output_get_3 (Variables|Default|SetAttemptsLosePoint (Utilities|Array|MakeArray (Variables|Default|GetTerminal_Unreal_With_MiniGame_Loss_Point_1) (Variables|Default|GetTerminal_Unreal_With_MiniGame_Loss_Point_2))))
  ;[1 1 1] Make array objects 0 scale
  (for _array_element _output_get
    (Transformation|SetWorldScale3D _array_element "0, 0, 0"))
  (for _array_element_2 _output_get_2
    (Transformation|SetWorldScale3D _array_element_2 "0, 0, 0"))
  (for _array_element_3 _output_get_3
    (Transformation|SetWorldScale3D _array_element_3 "0, 0, 0")))

(event Collision|EventActorBeginOverlap
  (params (OtherActor :type Actor%20Object%20Reference))
  ;[1 1 1] Gets player controller from actor using player Index
  (if (not (Variables|Default|GetSTOP))
    (if (Actor|ActorHasTag OtherActor "Player")
      (bind _output_get (Variables|Default|SetplayerActorReference OtherActor))
      (Variables|Default|SetplayerControllerReference (Game|GetPlayerController (Math|Conversions|ToInteger(Byte) (Utilities|String|GetSubstring (Utilities|GetObjectName _output_get) 26))))
      (Variables|Default|SetaccessTerminal true))))

(event EventTick
  (params (DeltaSeconds :type Float%20%28single-precision%29))
  (bind _scalearrayobjtimeline (Variables|Default|GetScaleArrayObjTimeLine))
  (bind _playercontrollerreference (Variables|Default|GetplayerControllerReference))
  (Utilities|FlowControl|Sequence
    (:then_1
      (if (not (Variables|Default|GetSTOP))
        (if (Variables|Default|GetaccessTerminal)
          (if (Variables|Default|GetMiniGamePlay)
            (CallFunction|ServerSide false true)
            (CallFunction|Minigame true)
            (else
              ;[1 1 1] Playing MiniGame after using for X duration
              (Variables|Default|SetArrayScaleDone false)
              (Utilities|IsValid _playercontrollerreference
                (:Is%20Valid
                  (if (Game|Player|IsInputKeyDown _playercontrollerreference (Variables|Default|GetuseKey))
                    (CallFunction|ServerSide true false)
                    (CallFunction|InputDelay true))))))
          (elif (not (Variables|Default|GetArrayScaleDone))
            (if (not (Audio|Components|Audio|IsPlaying _scalearrayobjtimeline))
              (Utilities|String|Reverse _scalearrayobjtimeline))))))))

(event Collision|EventActorEndOverlap
  (params (OtherActor :type Actor%20Object%20Reference))
  ;[1 1 1] Resets Variables
  (Variables|Default|SetMiniGamePlay false)
  (Variables|Default|SetArrayScaleDone false)
  (Variables|Default|SetObjScaleDone false)
  (Variables|Default|SetaccessTerminal false)
  (Variables|Default|SetplayerControllerReference 0)
  (Variables|Default|SetplayerActorReference 0)
  (Variables|Default|SetcurrentCompletion 0.0)
  (Components|Activation|Deactivate (Variables|Default|GetCamera)))

(fn ConstructionScript)

(fn ArrayLerpScaleDown
  (params (ArrayToLerp :type Array%20of%20Static%20Mesh%20Component%20Object%20References))
  (for _array_element ArrayToLerp
    (Transformation|SetWorldScale3D _array_element (Math|Vector|Lerp(Vector) (Transformation|GetWorldScale _array_element) "0, 0, 0" (* (Utilities|Time|GetWorldDeltaSeconds) 0.8)))
    (if (<= (.X (Class|KismetMathLibrary|BreakVector3f (Transformation|GetWorldScale _array_element))) 0.05)
      (Transformation|SetWorldScale3D _array_element "0, 0, 0")))
  (return))

(fn LerpManyArrayDown
  (CallFunction|ArrayLerpScaleDown (Variables|Default|GetTerminalComponent)))

(fn CheckPointerRottoTarget
  (bind _singleitemscaletimeline (Variables|Default|GetSingleItemScaleTimeLine))
  (bind _angleoftolerance (Variables|Default|GetAngleOfTolerance))
  (bind _terminal_unreal_with_minigame_pointer (Variables|Default|GetTerminal_Unreal_With_MiniGame_Pointer))
  (bind _terminal_unreal_with_minigame_target (Variables|Default|GetTerminal_Unreal_With_MiniGame_Target))
  (bind _singleitemscaletimeline_2 (Variables|Default|GetSingleItemScaleTimeLine))
  (bind _relativerotation (Variables|/Script/Engine.SceneComponent|GetRelativeRotation _terminal_unreal_with_minigame_pointer))
  (bind _relativerotation_2 (Variables|/Script/Engine.SceneComponent|GetRelativeRotation _terminal_unreal_with_minigame_target))
  (bind _returnvalue (- (.yaw _relativerotation_2) (.yaw _relativerotation)))
  (bind _returnvalue_2 (Math|Float|Absolute(Float) _returnvalue))
  (bind _returnvalue_3 (- 3.6e+02 _returnvalue_2))
  (if (Math|Boolean|ORBoolean (<= (Math|Float|Absolute(Float) _returnvalue_3) _angleoftolerance) (<= _returnvalue_3 _angleoftolerance) (<= _returnvalue_2 (Variables|Default|GetAngleOfTolerance)))
    ;[1 1 1] Scale Outcome Point
    (if (Variables|Default|GetObjScaleDone)
      ;[1 1 1] Wins 1 round of mini game
      (Variables|Default|SetWins (+ (Variables|Default|GetWins) 1))
      (return)
      (elif (not (Audio|Components|Audio|IsPlaying _singleitemscaletimeline))
        (Variables|Default|SetObjToScale (Utilities|Array|Get(acopy) (Variables|Default|GetAttemptsWinPoint) (Variables|Default|GetWins)))
        (Components|Timeline|PlayfromStart _singleitemscaletimeline)))
    (elif (Variables|Default|GetObjScaleDone)
      ;[1 1 1] loses 1 round of mini game
      (Variables|Default|SetLoss (+ (Variables|Default|GetLoss) 1))
      (return)
      (elif (not (Audio|Components|Audio|IsPlaying _singleitemscaletimeline_2))
        (Variables|Default|SetObjToScale (Utilities|Array|Get(acopy) (Variables|Default|GetAttemptsLosePoint) (Variables|Default|GetLoss)))
        (Components|Timeline|PlayfromStart _singleitemscaletimeline_2)))))

(fn 1RoundMiniGameClockWise
  (bind _pointertimeline (Variables|Default|GetPointerTimeLine))
  (bind _playercontrollerreference (Variables|Default|GetplayerControllerReference))
  (bind _targettimeline (Variables|Default|GetTargetTimeLine))
  (if (Variables|Default|Gettarget%20Set)
    (Utilities|IsValid _playercontrollerreference
      (:Is%20Valid
        (if (or (Game|Player|IsInputKeyDown _playercontrollerreference (Variables|Default|GetuseKey)) (Variables|Default|GetPressed))
          ;[1 1 1] Stop point rot and check outcome
          (Audio|Components|Audio|Stop _pointertimeline)
          (Variables|Default|SetPressed true)
          (CallFunction|CheckPointerRottoTarget)
          (else
            ;[1 1 1] Rotate Pointer
            (if (not (Audio|Components|Audio|IsPlaying _pointertimeline))
              (Variables|Default|SetReverse false)
              (Components|Timeline|PlayfromStart _pointertimeline))))))
    (else
      ;[1 1 1] Set Target Pos
      (if (not (Audio|Components|Audio|IsPlaying _targettimeline))
        (Transformation|SetRelativeRotation (Variables|Default|GetTerminal_Unreal_With_MiniGame_Target) "0, 0, 0" false false)
        (Components|Timeline|PlayfromStart _targettimeline)))))

(fn 1RoundMiniGameAntiClockWise
  (bind _pointertimeline (Variables|Default|GetPointerTimeLine))
  (bind _playercontrollerreference (Variables|Default|GetplayerControllerReference))
  (bind _targettimeline (Variables|Default|GetTargetTimeLine))
  (if (Variables|Default|Gettarget%20Set)
    (Utilities|IsValid _playercontrollerreference
      (:Is%20Valid
        (if (or (Game|Player|IsInputKeyDown _playercontrollerreference (Variables|Default|GetuseKey)) (Variables|Default|GetPressed))
          (Audio|Components|Audio|Stop _pointertimeline)
          (Variables|Default|SetPressed true)
          (CallFunction|CheckPointerRottoTarget)
          (elif (not (Audio|Components|Audio|IsPlaying _pointertimeline))
            (Variables|Default|SetReverse true)
            (Components|Timeline|PlayfromStart _pointertimeline)))))
    (elif (not (Audio|Components|Audio|IsPlaying _targettimeline))
      (Transformation|SetRelativeRotation (Variables|Default|GetTerminal_Unreal_With_MiniGame_Target) "0, 0, 0" false false)
      (Components|Timeline|PlayfromStart _targettimeline))))