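; BP_MainLabDoor is the main lab door, meant to unlock once every terminal in the level has been unlocked.
; On BeginPlay it gathers actors tagged "Terminal" and stores their count as the target.
; TellTerminalIsUnlocked increments an unlocked counter, which Tick compares to that target every frame.
; A match sets UnlockMainDoor, but the following branch is empty, so no opening behavior is implemented here.
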(event EventBeginPlay
  (bind _outactors (Actor|GetAllActorswithTag "Terminal"))
  (bind _output_get (Variables|Default|SetTerminals _outactors))
  (Variables|Default|SetmaxTerminalToUnlock (Utilities|Array|Length _output_get)))

(event Collision|EventActorBeginOverlap
  (params (OtherActor :type Actor%20Object%20Reference)))

(event EventTick
  (params (DeltaSeconds :type Float%20%28single-precision%29))
  ;[1 1 1] Check if door can be unlocked
  (Math|Integer|CompareInt (Variables|Default|GetterminalsUnlocked) (Variables|Default|GetmaxTerminalToUnlock)
    (:==
      (bind _output_get (Variables|Default|SetunlockMainDoor true))
      (if _output_get
        _))))

(fn ConstructionScript)

(fn TellTerminalIsUnlocked
  ;[1 1 1] Increase unlocked terminal Var
  (Variables|Default|SetterminalsUnlocked (+ (Variables|Default|GetterminalsUnlocked) 1)))